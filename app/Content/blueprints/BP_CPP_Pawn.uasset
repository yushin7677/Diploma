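; BP_CPP_Pawn is an AR pawn that simulates radiation exposure based on its position in the world.
; On BeginPlay it starts an AR session and adds a UI widget to the viewport.
; Each tick it passes its truncated integer location to GetFuflo, scales the result down into Radiation, and integrates that over delta time into a running Dose.
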(event `self.ReceiveBeginPlay`
  (`ARBlueprintLibrary.StartARSession` "/Game/blueprints/AR1.AR1")
  (bind _returnvalue (`|CreateWidget` "/Game/UI/UI.UI_C"))
  (`UserWidget.AddToViewport` _returnvalue 0))

(event `self.ReceiveTick`
  (params (DeltaSeconds :type "Float (single-precision)"))
  (bind (_returnvalue_x _returnvalue_y _returnvalue_z) (`KismetMathLibrary.BreakVector` (`self.K2_GetActorLocation`)))
  (bind _returnvalue (`self.getFuflo` (`KismetMathLibrary.FTrunc` _returnvalue_x) (`KismetMathLibrary.FTrunc` _returnvalue_y) (`KismetMathLibrary.FTrunc` _returnvalue_z)))
  (bind _output_get (set `self.radiation` (/ (`KismetMathLibrary.Conv_IntToDouble` _returnvalue) 100.0)))
  (set `self.dose` (+ (`self.dose`) (* _output_get (`GameplayStatics.GetWorldDeltaSeconds`)))))

(fn `UserConstructionScript`)